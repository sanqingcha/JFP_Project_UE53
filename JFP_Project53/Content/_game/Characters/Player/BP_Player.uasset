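; Player Blueprint that shows a Paper2D flipbook whose sprite, size and position change with a Jump or Hide state and a five-step level.
; PlayAnimation picks scale and offset, then SetState swaps the flipbook by level and Tstate and moves the actor relative to its BeginPlay location.
; When Tstate is false, Jump also replays a double-speed timeline that offsets the flipbook in X and Z for a hop.
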(event Custom|PlayAnimation
  (params (tstate :type Boolean) (Level :type Integer) (State :type E_TreeState%20Enum :default "NewEnumerator0"))
  (switch Utilities|FlowControl|Switch|SwitchonE_TreeState State
    (:NewEnumerator0
      (if tstate
        (CallFunction|SetState (Utilities|Select :Index Level :Option%200 0.7 :Option%201 1.0 :Option%202 1.5 :Option%203 2.2 :Option%204 3.0) tstate Level "NewEnumerator0" (Utilities|Select :Index Level :Option%200 "0.000000,0.000000,2.000000" :Option%201 "0.000000,0.000000,10.000000" :Option%202 "0.000000,0.000000,20.000000" :Option%203 "0.000000,0.000000,23.000000" :Option%204 "5.000000,0.000000,35.000000") :!label _label)
        (else
          (Utilities|FlowControl|Sequence
            (:then_0
              (goto _label))
            (:then_1
              (Components|Timeline|SetPlayRate (Variables|Default|GetJumpAnimation) 2.0)
              (bind (_direction _jumpline _r_l_line) (Timeline|JumpAnimation PlayFromStart)
                (:Update
                  (Transformation|SetRelativeLocation (Variables|Default|GetPaperFlipbook) (Math|Vector|MakeVector (Math|Float|Lerp -1.0 1.0 _r_l_line) 0.0 (Math|Float|Lerp 0.0 5.0 _jumpline)) false false))))))))
    (:NewEnumerator6
      (CallFunction|SetState 0.5 false 0 "NewEnumerator6" "0.000000,0.000000,8.000000"))))

(event EventBeginPlay
  (Utilities|FlowControl|Sequence
    (:then_0
      (CallFunction|InitialPawn))))

(fn ConstructionScript)

(fn InitialPawn
  (Variables|Default|SetFirstLocation (Transformation|GetActorLocation)))

(fn SetState
  (params (Scale :type Float%20%28double-precision%29) (tState :type Boolean) (Level :type Integer) (State :type E_TreeState%20Enum :default "NewEnumerator0") (OffestLocation :type Vector))
  (bind _paperflipbook (Variables|Default|GetPaperFlipbook))
  (switch Utilities|FlowControl|Switch|SwitchonE_TreeState State
    (:NewEnumerator0
      (switch int Level
        (:0
          (if tState
            (Sprite|SetFlipbook _paperflipbook "/Game/_game/Tex/Player/tree.tree")
            (else
              (Sprite|SetFlipbook _paperflipbook "/Game/_game/Tex/Player/tree.tree"))))
        (:1
          (if tState
            (Sprite|SetFlipbook _paperflipbook "/Game/_game/Tex/Player/tree2.tree2")
            (else
              (Sprite|SetFlipbook _paperflipbook "/Game/_game/Tex/Player/tree1.tree1"))))
        (:2
          (if tState
            (Sprite|SetFlipbook _paperflipbook "/Game/_game/Tex/Player/tree3.tree3")
            (else
              (Sprite|SetFlipbook _paperflipbook "/Game/_game/Tex/Player/tree4.tree4"))))
        (:3
          (if tState
            (Sprite|SetFlipbook _paperflipbook "/Game/_game/Tex/Player/tree5.tree5")
            (else
              (Sprite|SetFlipbook _paperflipbook "/Game/_game/Tex/Player/tree6.tree6"))))
        (:4
          (if tState
            (Sprite|SetFlipbook _paperflipbook "/Game/_game/Tex/Player/tree7.tree7")
            (else
              (Sprite|SetFlipbook _paperflipbook "/Game/_game/Tex/Player/tree7.tree7"))))))
    (:NewEnumerator6
      (Sprite|SetFlipbook _paperflipbook "/Game/_game/Tex/Player/HS.HS")))
  (Transformation|SetRelativeScale3D (Variables|Default|GetPaperFlipbook) (* (Variables|Default|GetScale) Scale))
  (Transformation|SetActorLocation (+ OffestLocation (Variables|Default|GetFirstLocation)) false false))