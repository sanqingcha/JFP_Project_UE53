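; Player controller for a nutrient-gathering survival game: it possesses BP_Player, spawns the camera, creates HUD widgets and handles gather and hide input.
; Gathering raises nutrient and levels up toward victory and the story level, while a looping timer drains it until death.
; BPICheck kills the player when not hidden.
; BP_manager events gate a tutorial stage, unlocking hiding, then lifting the nutrient clamps via StageOk.
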(event Custom|StoryDelay
  (Utilities|FlowControl|Delay 2.0)
  (Game|OpenLevel(byObjectReference) "/Game/_game/Map/StoryMap/Level_Story.Level_Story"))

(event EventBPICheck
  (if (not (.hide (Variables|Default|GetPlayerState_t)))
    (Utilities|FlowControl|DoOnce false
      (:Completed
        (CallFunction|Dead true)))))

(event EventBeginPlay
  (Utilities|FlowControl|Sequence
    (:then_1
      (CallFunction|ContorllPlayer))
    (:then_2
      (CallFunction|SpawnCamera))
    (:then_3
      (CallFunction|GetGameHUD))
    (:then_4
      (CallFunction|Initial))
    (:then_5
      (CallFunction|ActionInitial))))

(event Custom|ActionInitial
  (bind _self self)
  (bind _returnvalue (PlayerController|LocalPlayerSubsystems|GetEnhancedInputLocalPlayerSubsystem _self))
  (Utilities|IsValid _returnvalue
    (:Is%20Valid
      (Input|AddMappingContext _returnvalue "/Game/_game/Characters/Player/Input/IM_Player.IM_Player" 0 "(bIgnoreAllPressedKeysUntilRelease=True,bForceImmediately=False,bNotifyUserSettings=False)")
      (bind _returnvalue_2 (Utilities|Time|SetTimerbyFunctionName 0 "Sub_nutrient" (Variables|Default|GetTimedurition) true))
      (Variables|Default|SetTimeHandle _returnvalue_2))))

(event Custom|OKl
  (Variables|Default|SetStagH true)
  (Class|BPIWBTips|BPISetVis(Message) (Variables|Default|GetWB_Tips) false false true)
  (Utilities|FlowControl|DoOnce true) ; enters at Reset
)

(event Custom|Over
  (Default|StartShow (Variables|Default|GetManager))
  (Variables|Default|SetStageOk true))

(event Input|EnhancedActionEvents|EnhancedInputActionIA_get_nutrient
  (params (ActionValue :type Boolean) (ElapsedSeconds :type Float%20%28double-precision%29) (TriggeredSeconds :type Float%20%28double-precision%29) (InputAction :type Input%20Action%20Object%20Reference :default "/Game/_game/Characters/Player/Input/Action/IA_get_nutrient.IA_get_nutrient"))
  (bind _manager (Variables|Default|GetManager))
  (:Started
    (if (not (.dead (Variables|Default|GetPlayerState_t)))
      (Utilities|Struct|SetmembersinST_PlayerState (Variables|Default|GetPlayerState_t) false)
      (CallFunction|AddNutrient)
      (Default|PlayAnimation (Variables|Default|GetBP_Pawn) false (.current_level (Variables|Default|GetState_nutrient)) "NewEnumerator0")
      (Timeline|GetBackLine PlayFromStart
        (:Finished
          (if (not (.hide (Variables|Default|GetPlayerState_t)))
            (Default|PlayAnimation (Variables|Default|GetBP_Pawn) true (.current_level (Variables|Default|GetState_nutrient)) "NewEnumerator0")
            (Utilities|FlowControl|DoOnce false
              (:Completed
                (Class|BPIWBTips|BPISetVis(Message) (Variables|Default|GetWB_Tips) false false false)
                (Utilities|FlowControl|Sequence
                  (:then_0
                    (Default|Showstate01 _manager)
                    (EventDispatchers|BindEventtoOKl _manager (delegate Custom|OKl))
                    (EventDispatchers|BindEventtoOver _manager (delegate Custom|Over))))))))))))

(event Input|EnhancedActionEvents|EnhancedInputActionIA_Hide
  (params (ActionValue :type Boolean) (ElapsedSeconds :type Float%20%28double-precision%29) (TriggeredSeconds :type Float%20%28double-precision%29) (InputAction :type Input%20Action%20Object%20Reference :default "/Game/_game/Characters/Player/Input/Action/IA_Hide.IA_Hide"))
  (bind _playerstate_t (Variables|Default|GetPlayerState_t))
  (:Started
    (if (Variables|Default|GetStagH)
      (if (not (or (.dead _playerstate_t) (.victory _playerstate_t)))
        (Default|PlayAnimation (Variables|Default|GetBP_Pawn) false 0 "NewEnumerator6")
        (Utilities|Struct|SetmembersinST_PlayerState (Variables|Default|GetPlayerState_t) true)
        (Utilities|FlowControl|DoOnce true
          (:Completed
            (Class|BPIWBTips|BPISetVis(Message) (Variables|Default|GetWB_Tips) false true false)))))))

(fn ConstructionScript)

(fn Initial
  (bind _state_nutrient (Variables|Default|GetState_nutrient))
  (Utilities|Struct|SetmembersinST_nutrient (Variables|Default|GetState_nutrient) (Utilities|Array|Get(acopy) (.levelfirstnutrient _state_nutrient)) (Utilities|Array|Get(acopy) (.add_nutrients _state_nutrient)))
  (Variables|Default|SetbShowMouseCursor true)
  (bind _wb (Class|BPIHUD|BPICreatWB(Message) (Variables|Default|GetHUD) "/Game/_game/UI/GameUI/WB_Return.WB_Return_C" 0 "WB_Return" "Visible" 10))
  (Variables|Default|SetReturn _wb)
  (bind _wb_2 (Class|BPIHUD|BPICreatWB(Message) (Variables|Default|GetHUD) "/Game/_game/UI/Tips/WB_Tips.WB_Tips_C" 0 "WB_Tips" "Visible" -1))
  (Variables|Default|SetWB_Tips _wb_2)
  (Class|BPIWBTips|BPIStartSai(Message) _wb_2)
  (Class|BPIWBTips|BPISetVis(Message) _wb_2 true false false)
  (bind _returnvalue (Actor|GetActorOfClass "/Game/_game/BP_manager.BP_manager_C"))
  (Variables|Default|SetManager _returnvalue))

(fn SpawnCamera
  (bind _returnvalue (Game|SpawnActorfromClass "/Game/_game/Characters/Player/Camera/BP_Camera.BP_Camera_C" (Math|Transform|MakeTransform "0, 0, 0" "0, 0, 0" "1.000000,1.000000,1.000000") "Undefined" "MultiplyWithRoot" 0 0))
  (Game|Player|SetViewTargetwithBlend _returnvalue 0.0 "VTBlend_Linear" 0.0 false))

(fn GetGameHUD
  (Variables|Default|SetHUD (HUD|GetHUD)))

(fn AddNutrient
  (bind _state_nutrient (Variables|Default|GetState_nutrient))
  (bind _stageok (Variables|Default|GetStageOk))
  (bind _state_nutrient_2 (Variables|Default|GetState_nutrient))
  (bind _state_nutrient_3 (Variables|Default|GetState_nutrient))
  (bind _returnvalue (+ (.current_nutrient _state_nutrient_2) (.add_nutrient _state_nutrient_2)))
  (bind _returnvalue_2 (Math|Float|Clamp(Float) _returnvalue 0.0 6e+01))
  (bind _returnvalue_3 (Math|Float|SelectFloat _returnvalue _returnvalue_2 _stageok))
  (Variables|Default|GetStaticWB%20Nutrient
    (:then
      (if (>= _returnvalue_3 (.max_nutrient _state_nutrient_2))
        (Utilities|Struct|SetmembersinST_nutrient (Variables|Default|GetState_nutrient) (.max_nutrient _state_nutrient_2))
        (Utilities|FlowControl|Sequence
          (:then_0
            (Default|SetPercent (Variables|Default|GetStaticWB%20Nutrient) (/ (.current_nutrient _state_nutrient_3) (.max_nutrient _state_nutrient_3)) :!label _label))
          (:then_1
            (bind _output_get (LocalVariables|SetLevel (+ (.current_level _state_nutrient) 1)))
            (if (>= _output_get (.maxlevel _state_nutrient))
              (CallFunction|Victory)
              (Utilities|Struct|SetmembersinST_nutrient (Variables|Default|GetState_nutrient) 1e+02 (LocalVariables|GetLevel))
              (else
                (CallFunction|AddLevel)
                (Utilities|Struct|SetmembersinST_nutrient (Variables|Default|GetState_nutrient) (Utilities|Array|Get(acopy) (.levelfirstnutrient (Variables|Default|GetState_nutrient)) (LocalVariables|GetLevel)) (LocalVariables|GetLevel))
                (Variables|/Game/_game/BP_manager.BP_manager_C|SetLevelStatge (Variables|Default|GetManager) (LocalVariables|GetLevel))))))
        (else
          (Utilities|Struct|SetmembersinST_nutrient (Variables|Default|GetState_nutrient) _returnvalue_3)
          (goto _label))))
    (:else)))

(fn SubNutrient
  (bind _timedurition (Variables|Default|GetTimedurition))
  (bind _state_nutrient (Variables|Default|GetState_nutrient))
  (bind _state_nutrient_2 (Variables|Default|GetState_nutrient))
  (bind _stageok (Variables|Default|GetStageOk))
  (bind _output (Utilities|Array|Get(acopy) (.sub_nutrient _state_nutrient) (.current_level _state_nutrient)))
  (bind _returnvalue (* _timedurition _output))
  (bind _returnvalue_2 (- (.current_nutrient _state_nutrient) _returnvalue))
  (bind _returnvalue_3 (Math|Float|Clamp(Float) _returnvalue_2 1e+01 1e+02))
  (bind _returnvalue_4 (Math|Float|SelectFloat _returnvalue_2 _returnvalue_3 _stageok))
  (if (<= _returnvalue_4 0.0)
    (Utilities|Struct|SetmembersinST_nutrient (Variables|Default|GetState_nutrient) 0.0)
    (Utilities|FlowControl|Sequence
      (:then_0
        (CallFunction|Dead false))
      (:then_1
        (bind _staticwb_nutrient (Variables|Default|GetStaticWB%20Nutrient :!label _label)
          (:then
            _)
          (:else
            (bind _wb (Class|BPIHUD|BPIGetWB(Message) (Variables|Default|GetHUD) "WB_nutrient"))
            (bind _aswb_nutrient (Utilities|Casting|CastToWB_nutrient _wb))
            (Variables|Default|SetStaticWB%20Nutrient _aswb_nutrient)))
        (Default|SetPercent _staticwb_nutrient (/ (.current_nutrient _state_nutrient_2) (.max_nutrient _state_nutrient_2)))))
    (else
      (Utilities|Struct|SetmembersinST_nutrient (Variables|Default|GetState_nutrient) _returnvalue_4)
      (goto _label))))

(fn Victory
  (bind _playerstate_t (Variables|Default|GetPlayerState_t))
  (bind _manager (Variables|Default|GetManager))
  (Utilities|FlowControl|DoOnce false
    (:Completed
      (Utilities|Time|ClearandInvalidateTimerbyHandle (Variables|Default|GetTimeHandle))
      (Utilities|Struct|SetmembersinST_PlayerState _playerstate_t (.Hide (Utilities|Struct|BreakST_PlayerState _playerstate_t)) false true)
      (Variables|/Game/_game/BP_manager.BP_manager_C|SetVictor _manager true)
      (Default|Show _manager)
      (Variables|/Game/_game/GI_Game.GI_Game_C|SetEnd? (CallFunction|GetGameGI) true)
      (CallFunction|StoryDelay))))

(fn Dead
  (params (BeDestory :type Boolean))
  (bind _hud (Variables|Default|GetHUD))
  (Utilities|Time|ClearandInvalidateTimerbyHandle (Variables|Default|GetTimeHandle))
  (Utilities|Struct|SetmembersinST_PlayerState (Variables|Default|GetPlayerState_t) true)
  (Default|PlayAnimation (Variables|Default|GetBP_Pawn) false 0 "NewEnumerator1")
  (Class|BPIHUD|BPICreatWB(Message) _hud "/Game/_game/UI/MainMenu/WB_Dead.WB_Dead_C" 0 "WB_Dead" "Visible")
  (bind _wb (Class|BPIHUD|BPIGetWB(Message) _hud "WB_Dead"))
  (Class|BPIWBDead|BPIPlayerAnimation(Message) _wb BeDestory)
  (Variables|Default|SetbShowMouseCursor true)
  (Widget|RemovefromParent (Variables|Default|GetReturn)))

(fn ContorllPlayer
  (bind _returnvalue (Actor|GetActorOfClass "/Game/_game/Characters/Player/BP_Player.BP_Player_C"))
  (bind _output_get (Variables|Default|SetBP_Pawn _returnvalue))
  (Pawn|Possess _output_get))

(fn AddLevel
  (bind _state_nutrient (Variables|Default|GetState_nutrient))
  (Utilities|Struct|SetmembersinST_nutrient (Variables|Default|GetState_nutrient) (Utilities|Array|Get(acopy) (.add_nutrients _state_nutrient) (.current_level _state_nutrient))))