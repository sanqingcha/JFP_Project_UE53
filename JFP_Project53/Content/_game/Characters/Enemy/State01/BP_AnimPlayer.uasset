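; Enemy state animation actor that plays a timed tip-then-check sequence with two planes, signalling the player controller during the check.
; Start scales timelines from TipsTime and Detime: one plane rotates, then another slides out, holds and reverses at a random rate.
; A one-shot macro gate stops the reversed timeline retriggering the hold.
; Tick sends BPICheckMessage while the slide timeline's CheckTime track flags Checking, unless ShowOnly is set.
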(event Custom|Start
  (params (detime :type Float%20%28double-precision%29) (tipsTime :type Float%20%28double-precision%29) (showOnly :type Boolean))
  (Variables|Default|SetShow%20Only showOnly)
  (CallFunction|Animation1 detime tipsTime))

(event Custom|Animation1
  (params (detime :type Float%20%28double-precision%29) (TipsTime :type Float%20%28double-precision%29))
  (bind _returnvalue (< detime 2.0))
  (Variables|Default|SetAnimiation01Rate (/ 2.5 (Math|Float|Clamp(Float) TipsTime 1e-05 1e+04)))
  (Variables|Default|SetPlayRate (Math|Float|SelectFloat 0.0 (Math|Float|SelectFloat (/ 2.0 (Math|Float|Clamp(Float) detime 0.0001 1e+03)) 1.0 _returnvalue) (== detime 0.0)))
  (Variables|Default|SetDisTime (Math|Float|SelectFloat 0.0 (- detime 2.0) _returnvalue))
  (Utilities|FlowControl|Sequence
    (:then_1
      (Components|Timeline|SetPlayRate (Variables|Default|GetAnimation1_Line) (Variables|Default|GetAnimiation01Rate))
      (bind _anim01 (Timeline|Animation1_Line PlayFromStart)
        (:Update
          (Transformation|SetRelativeRotation (Variables|Default|GetPlane) (Math|Rotator|Lerp(Rotator) "-95.000000,-90.000000,90.000000" "14.000000,-90.000000,90.000000" _anim01) false false))
        (:Finished
          (CallFunction|Animation2))))))

(event Custom|Animation2
  (Utilities|FlowControl|Sequence
    (:then_0
      (Components|Timeline|SetPlayRate (Variables|Default|GetAnimation23_line) (Variables|Default|GetPlayRate))
      (bind (_direction _anim01 _checktime) (Timeline|Animation23_line PlayFromStart)
        (:Update
          (Transformation|SetRelativeLocation (Variables|Default|GetPlane1) (Math|Vector|Lerp(Vector) "-7.000000,-37.432172,60.512839" "-7.000000,40.365236,64.057310" _anim01) false false)
          (if (> _checktime 1.0)
            (Variables|Default|SetChecking true)
            (else
              (Variables|Default|SetChecking false))))
        (:Finished
          (Utilities|OpenExc :!label _label
            (:output
              (Utilities|FlowControl|Delay (Variables|Default|GetDisTime))
              (CallFunction|Animation03))))))
    (:then_1
      (goto _label Open))))

(event Custom|Animation03
  (Components|Timeline|SetPlayRate (Variables|Default|GetAnimation23_line) (Math|Random|RandomFloatinRange 1.0 (Variables|Default|GetPlayRate)))
  (bind (_direction _anim01 _checktime) (Timeline|Animation23_line ReverseFromEnd)
    (:Update
      (Transformation|SetRelativeLocation (Variables|Default|GetPlane1) (Math|Vector|Lerp(Vector) "-7.000000,-37.432172,60.512839" "-7.000000,40.365236,64.057310" _anim01) false false)
      (if (> _checktime 1.0)
        (Variables|Default|SetChecking true)
        (else
          (Variables|Default|SetChecking false))))
    (:Finished
      (Utilities|OpenExc
        (:output
          (Utilities|FlowControl|Delay (Variables|Default|GetDisTime))
          (CallFunction|Animation03))))))

(event EventTick
  (params (DeltaSeconds :type Float%20%28single-precision%29))
  (if (and (not (Variables|Default|GetShow%20Only)) (Variables|Default|GetChecking))
    (Class|BPIPC|BPICheck(Message) (Game|GetPlayerController 0))))

(fn ConstructionScript)