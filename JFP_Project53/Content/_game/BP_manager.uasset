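; BP_manager schedules timed shows on the BP_AnimPlayer actor it finds at BeginPlay.
; showstate01 plays one fixed-timing show bracketed by CallOKl and CallOver, while Show starts a long show-only display.
; StartShow loops the latent Action routine until Victor is set, randomizing delays, duration and tip time within ranges selected by LevelStatge.
; Action waits, starts the anim player, then holds until that round ends.
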(event Custom|StartShow
  (bind _levelstatge (Variables|Default|GetLevelStatge))
  (bind _levelstatge_2 (Variables|Default|GetLevelStatge))
  (bind _levelstatge_3 (Variables|Default|GetLevelStatge))
  (bind _returnvalue (Utilities|Select :Index _levelstatge :Option%200 2.0 :Option%201 2.0 :Option%202 2.0 :Option%203 0.5))
  (bind _returnvalue_2 (Utilities|Select :Index _levelstatge :Option%200 2.0 :Option%201 2.0 :Option%202 2.0 :Option%203 1.0))
  (bind _returnvalue_3 (Math|Random|RandomFloatinRange _returnvalue _returnvalue_2))
  (if (not (Variables|Default|GetVictor)) :!label _label
    (Utilities|Action _returnvalue_3 (Math|Random|RandomFloatinRange (Utilities|Select :Index _levelstatge_2 :Option%200 3.0 :Option%201 2.0 :Option%202 1.0 :Option%203 3.0) (Utilities|Select :Index _levelstatge_2 :Option%200 4.0 :Option%201 3.0 :Option%202 2.0 :Option%203 5.0)) _returnvalue_3 (Math|Random|RandomFloatinRange (Utilities|Select :Index _levelstatge_3 :Option%200 2.5 :Option%201 1.5 :Option%202 0.5 :Option%203 0.1) (Utilities|Select :Index _levelstatge_3 :Option%200 3.5 :Option%201 2.5 :Option%202 1.5 :Option%203 1.0)) (Variables|Default|GetVictor) false)
    (goto _label)))

(event Custom|Show
  (Utilities|Action 0.0 1e+04 0.0 0.0 false true))

(event Custom|showstate01
  (Utilities|FlowControl|Delay 2.0)
  (Default|CallOKl)
  (Default|Start (Variables|Default|GetAnimActor) 2.0 3.0 false)
  (Utilities|FlowControl|Delay 6.0)
  (Default|CallOver))

(event EventBeginPlay
  (bind _returnvalue (Actor|GetActorOfClass "/Game/_game/Characters/Enemy/State01/BP_AnimPlayer.BP_AnimPlayer_C"))
  (Variables|Default|SetAnimActor _returnvalue))

(fn ConstructionScript)